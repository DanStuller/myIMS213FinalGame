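; BP_Door is a door that swings open once enough items have been collected.
; CollectItem increments a counter, and OpenDoorCheck compares it to MaxItemCollected, firing OpenDoor only once through a DoOnce.
; OpenDoor plays a timeline whose DoorRotation track lerps the Door component's yaw to the open angle.
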(event `Open Door`
  (bind (_direction _door_rotation) (`Timeline|OpenDoor`)
    (:`Update`
      (`SceneComponent.K2_SetRelativeRotation` (`self.Door`) (`KismetMathLibrary.MakeRotator` 0.0 0.0 (`KismetMathLibrary.Lerp` 0.0 60.0 _door_rotation)) false false))))

(event `Collect Item`
  (`/Engine/EditorBlueprintResources/StandardMacros.IncrementInt` (`self.CurrentItemsCollected`)))

(event `Open Door Check`
  (if (>= (`self.CurrentItemsCollected`) (`self.MaxItemCollected`))
    (`/Engine/EditorBlueprintResources/StandardMacros.DoOnce` false
      (:`Completed`
        (`self.Open Door`)))))

(fn `UserConstructionScript`)